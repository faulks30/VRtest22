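; Game mode that, on BeginPlay, configures the player pawn for the current platform and builds the UI.
; It flags the DefaultPawn_BP for iOS or VR, and stops early if the player character is not that class.
; It adds the main HUD, plus an extra IOS_HUD on iOS, and creates a hidden MissionStatus widget.
; ToggleHUD shows or hides only that MissionStatus widget, tracking visibility with a boolean.
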(event EventBeginPlay
  (bind _returnvalue (Game|GetPlayerController 0))
  (bind _returnvalue_2 (Game|GetPlatformName))
  (bind _returnvalue_3 (Utilities|Enum|Equal(Enum) _returnvalue_2 "IOS"))
  ;[1 1 1] Create HUD, set platform variables
  (bind _asdefault_pawn_bp (Utilities|Casting|CastToDefaultPawn_BP (Game|GetPlayerCharacter 0)))
  (Variables|/Game/Blueprints/DefaultPawn_BP.DefaultPawn_BP_C|SetIOS%20Game _asdefault_pawn_bp _returnvalue_3)
  (Variables|/Game/Blueprints/DefaultPawn_BP.DefaultPawn_BP_C|SetVR%20Game _asdefault_pawn_bp (Class|HeadMountedDisplayFunctionLibrary|IsHeadMountedDisplayEnabled))
  (if _returnvalue_3
    (bind _returnvalue_4 (UserInterface|CreateWidget "/Game/Blueprints/UI/IOS_HUD.IOS_HUD_C" _returnvalue))
    (bind _output_get (Variables|Default|SetHUD_IOS_Widget _returnvalue_4))
    (UserInterface|Viewport|AddtoViewport _output_get 0))
  (bind _returnvalue_5 (UserInterface|CreateWidget "/Game/Blueprints/UI/HUD.HUD_C" _returnvalue))
  (bind _output_get_2 (Variables|Default|SetHUD_Widget _returnvalue_5))
  (UserInterface|Viewport|AddtoViewport _output_get_2 0)
  (bind _returnvalue_6 (UserInterface|CreateWidget "/Game/Blueprints/UI/MissionStatus.MissionStatus_C" _returnvalue))
  (Variables|Default|SetMS_widget _returnvalue_6)
  (Variables|Default|SetMS_Showing false))

(fn ConstructionScript)

(fn ToggleHUD
  (if (Variables|Default|GetMS_Showing)
    (Widget|RemovefromParent (Variables|Default|GetMS_widget))
    (Variables|Default|SetMS_Showing false)
    (else
      (UserInterface|Viewport|AddtoViewport (Variables|Default|GetMS_widget) 0)
      (Variables|Default|SetMS_Showing true))))