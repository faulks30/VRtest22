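; Player pawn for the sword character, extending a parent pawn with sword collision, cocking and supercharge state.
; Tick checks cocking, then on authority moves the sword collision parent to an interpolated transform and checks supercharge in combat mode.
; ShowHUD picks the VR HUD or builds base, sword, mission status and iOS widgets for the viewing player.
; HUDUpdateChar pushes sword speed, cocked and supercharged state to whichever HUD is active.
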(event EventBeginPlay
  ;[1 1 1] Begin Play - set PawnType 1 (Sword)
  (|CallParentFunction)
  (HUD|ShowHUD)
  (CallFunction|InitVRHUD))

(event EventTick
  (params (DeltaSeconds :type Float%20%28single-precision%29))
  ;[1 1 1] EVENT TICK - move the collision to the sword
  (|CallParentFunction DeltaSeconds)
  (CallFunction|CheckCockSword)
  (Networking|SwitchHasAuthority
    (:Authority
      (bind (_new_location _new_rotation) (CallFunction|InterpolateSword DeltaSeconds))
      (CallFunction|ServerSetLocationRotation (Variables|Default|GetSword%20Collision%20Parent) _new_location _new_rotation false false)
      (if (Variables|Default|GetCombat%20Mode)
        (CallFunction|CheckSwordSupercharged)))))

(fn ConstructionScript
  (|CallParentFunction))

(fn ShowHUD
  (bind _playercontroller (Variables|Default|GetPlayerController))
  (if (Variables|Default|GetVR%20Game)
    (CallFunction|ShowVRHUD)
    (else
      (CallFunction|HideVRHUD)
      (if (Variables|Default|GetIsViewingPlayer)
        (if (Variables|Default|GetIOS%20Game)
          (bind _returnvalue (UserInterface|CreateWidget "/Game/Blueprints/UI/IOS_HUD.IOS_HUD_C" _playercontroller))
          (bind _output_get (Variables|Default|SetHUD%20IOS%20Widget _returnvalue))
          (UserInterface|Viewport|AddtoViewport _output_get 0))
        (bind _returnvalue_2 (UserInterface|CreateWidget "/Game/Blueprints/UI/HUD.HUD_C" _playercontroller))
        (bind _output_get_2 (Variables|Default|SetHUD%20Base _returnvalue_2))
        (UserInterface|Viewport|AddtoViewport _output_get_2 0)
        (bind _returnvalue_3 (UserInterface|CreateWidget "/Game/Blueprints/UI/HUD_Sword.HUD_Sword_C" _playercontroller))
        (bind _output_get_3 (Variables|Default|SetHUD%20Character _returnvalue_3))
        (UserInterface|Viewport|AddtoViewport _output_get_3 0)
        (bind _returnvalue_4 (UserInterface|CreateWidget "/Game/Blueprints/UI/MissionStatus.MissionStatus_C" _playercontroller))
        (Variables|Default|SetMS%20Widget _returnvalue_4)
        (Variables|Default|SetMS%20Showing false)))))

(fn HUDUpdateChar
  (bind _hud_character (Variables|Default|GetHUD%20Character))
  (bind _sword_speed_max (Variables|Default|GetSword%20Speed%20Max))
  (bind _sword_speed (Variables|Default|GetSword%20Speed))
  (bind _sword_speed_over (Variables|Default|GetSword%20Speed%20Over))
  (bind _sword_supercharged (Variables|Default|GetSword%20Supercharged))
  (bind _sword_speed_max_2 (Variables|Default|GetSword%20Speed%20Max))
  (bind _returnvalue (/ _sword_speed _sword_speed_max))
  (bind _returnvalue_2 (/ _sword_speed_over _sword_speed_max_2))
  (if (Variables|Default|GetVR%20Game)
    (bind _ashud_vr (Utilities|Casting|CastToHUD_VR (UserInterface|GetUserWidgetObject (Variables|Default|GetWidget))))
    (bind _output_get (Variables|Default|SetHUD%20VR _ashud_vr))
    (Utilities|IsValid _output_get
      (:Is%20Valid
        (Variables|/Game/Blueprints/UI/HUD_VR.HUD_VR_C|SetSwordCocked (Variables|Default|GetHUD%20VR) (Variables|Default|GetSwordCocked))
        (Variables|/Game/Blueprints/UI/HUD_VR.HUD_VR_C|SetSwordSpeedVisible (Variables|Default|GetHUD%20VR) (Variables|Default|GetSwordSpeedVisible))
        (Progress|SetPercent (Variables|/Game/Blueprints/UI/HUD_VR.HUD_VR_C|GetSwordSpeed (Variables|Default|GetHUD%20VR)) _returnvalue)
        (Progress|SetPercent (Variables|/Game/Blueprints/UI/HUD_VR.HUD_VR_C|GetSwordSpeedOver (Variables|Default|GetHUD%20VR)) _returnvalue_2)
        (Variables|/Game/Blueprints/UI/HUD_VR.HUD_VR_C|SetSwordSuperCharged (Variables|Default|GetHUD%20VR) _sword_supercharged)))
    (else
      (Utilities|IsValid (Variables|Default|GetHUD%20Character)
        (:Is%20Valid
          (Variables|/Game/Blueprints/UI/HUD_Sword.HUD_Sword_C|SetSwordCocked _hud_character (Variables|Default|GetSwordCocked))
          (Variables|/Game/Blueprints/UI/HUD_Sword.HUD_Sword_C|SetSwordSpeedVisible _hud_character (Variables|Default|GetSwordSpeedVisible))
          (Progress|SetPercent (Variables|/Game/Blueprints/UI/HUD_Sword.HUD_Sword_C|GetSwordSpeed _hud_character) _returnvalue)
          (Progress|SetPercent (Variables|/Game/Blueprints/UI/HUD_Sword.HUD_Sword_C|GetSwordSpeedOver _hud_character) _returnvalue_2)
          (Variables|/Game/Blueprints/UI/HUD_Sword.HUD_Sword_C|SetSwordSuperCharged _hud_character _sword_supercharged)
          (return))))))