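; LobbyGM_BP is a lobby game mode with player spawning and a mission status toggle, though much of its setup is disconnected.
; RespawnPlayer spawns a DefaultPawn_BP at a random lobby spawn point and possesses it; its DestroyActor targets itself, not the old pawn.
; BeginPlay and PostLogin are empty, so the logic for spawn points, player registration, platform flags, HUD widgets and enemy lists never runs.
; ToggleHUD shows or hides MSWidget, whose creation is also disconnected.
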(event Custom|RespawnPlayer
  (params (PlayerController :type Player%20Controller%20BP%20Object%20Reference))
  (bind _lobbyspawnpoints (Variables|Default|GetLobbySpawnPoints))
  ;[1 1 1] Respawn new player
  (Utilities|IsValid (Pawn|GetControlledPawn PlayerController)
    (:Is%20Valid
      (Actor|DestroyActor))
    (:Is%20Not%20Valid
      _))
  (bind _returnvalue (Game|SpawnActorfromClass "/Game/Blueprints/DefaultPawn_BP.DefaultPawn_BP_C" (Transformation|GetActorTransform (Utilities|Array|Get(acopy) _lobbyspawnpoints (Math|Random|RandomIntegerinRange 0 (- (Utilities|Array|Length _lobbyspawnpoints) 1)))) "AdjustIfPossibleButAlwaysSpawn" 0 0))
  (Pawn|Possess PlayerController _returnvalue))

(event EventBeginPlay
  ;[1 1 1] Create HUD, set platform variables
)

(event EventPostLogin
  (params (NewPlayer :type Player%20Controller%20Object%20Reference))
  ;[1 1 1] New player logged on
)

(fn ConstructionScript)

(fn ToggleHUD
  (if (Variables|Default|GetMS_Showing)
    (Widget|RemovefromParent (Variables|Default|GetMS_widget))
    (Variables|Default|SetMS_Showing false)
    (else
      (UserInterface|Viewport|AddtoViewport (Variables|Default|GetMS_widget) 0)
      (Variables|Default|SetMS_Showing true))))