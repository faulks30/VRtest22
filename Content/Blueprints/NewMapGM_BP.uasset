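; Game mode that sets up the player UI and spawns players as they log in.
; BeginPlay flags iOS and VR on the pawn, creates platform-dependent HUDs and a toggleable mission status widget, and collects ClawZombie and QueenVampire enemies.
; On authority, PostLogin stores each controller and gathers PlayerStarts for RespawnPlayer, which spawns and possesses a pawn at a random one.
; If the controller already has a pawn, RespawnPlayer calls DestroyActor untargeted, hitting the game mode itself.
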(event Custom|RespawnPlayer
  (params (PlayerController :type Player%20Controller%20BP%20Object%20Reference))
  (bind _spawnpoints (Variables|Default|GetSpawnPoints))
  ;[1 1 1] Respawn new player
  (Utilities|IsValid (Pawn|GetControlledPawn PlayerController)
    (:Is%20Valid
      (Actor|DestroyActor))
    (:Is%20Not%20Valid
      _))
  (bind _returnvalue (Game|SpawnActorfromClass "/Game/Blueprints/DefaultPawn_BP.DefaultPawn_BP_C" (Transformation|GetActorTransform (Utilities|Array|Get(acopy) _spawnpoints (Math|Random|RandomIntegerinRange 0 (- (Utilities|Array|Length _spawnpoints) 1)))) "AdjustIfPossibleButAlwaysSpawn" 0 0))
  (Pawn|Possess PlayerController _returnvalue))

(event EventBeginPlay
  (bind _returnvalue (Game|GetPlayerController 0))
  (bind _returnvalue_2 (Game|GetPlatformName))
  (bind _returnvalue_3 (Class|HeadMountedDisplayFunctionLibrary|IsHeadMountedDisplayConnected))
  (bind _returnvalue_4 (Utilities|Enum|Equal(Enum) _returnvalue_2 "IOS"))
  ;[1 1 1] Create HUD, set platform variables
  (bind _asdefault_pawn_bp (Utilities|Casting|CastToDefaultPawn_BP (Game|GetPlayerCharacter 0)))
  (Variables|/Game/Blueprints/DefaultPawn_BP.DefaultPawn_BP_C|SetIOS%20Game _asdefault_pawn_bp _returnvalue_4)
  (Variables|/Game/Blueprints/DefaultPawn_BP.DefaultPawn_BP_C|SetVR%20Game _asdefault_pawn_bp _returnvalue_3)
  (if _returnvalue_4
    (bind _returnvalue_5 (UserInterface|CreateWidget "/Game/Blueprints/UI/IOS_HUD.IOS_HUD_C" _returnvalue))
    (bind _output_get (Variables|Default|SetHUD_IOS_Widget _returnvalue_5))
    (UserInterface|Viewport|AddtoViewport _output_get 0))
  (bind _returnvalue_6 (UserInterface|CreateWidget "/Game/Blueprints/UI/HUD.HUD_C" _returnvalue))
  (bind _output_get_2 (Variables|Default|SetHUD_Widget _returnvalue_6))
  (if _returnvalue_3
    _
    (else
      (UserInterface|Viewport|AddtoViewport _output_get_2 0)))
  (bind _returnvalue_7 (UserInterface|CreateWidget "/Game/Blueprints/UI/MissionStatus.MissionStatus_C" _returnvalue))
  (Variables|Default|SetMS_widget _returnvalue_7)
  (Variables|Default|SetMS_Showing false)
  (bind _outactors (Actor|GetAllActorsOfClass "/Game/Monsters/ClawZombie/ClawZombie.ClawZombie_C"))
  (Utilities|Array|AppendArray (Variables|Default|GetEnemy%20Actors) _outactors)
  (bind _outactors_2 (Actor|GetAllActorsOfClass "/Game/Monsters/QueenVampire/QueenVampire.QueenVampire_C"))
  (Utilities|Array|AppendArray (Variables|Default|GetEnemy%20Actors) _outactors_2))

(event EventPostLogin
  (params (NewPlayer :type Player%20Controller%20Object%20Reference))
  ;[1 1 1] New player logged on
  (Development|PrintString "Player Logged on")
  (Networking|SwitchHasAuthority
    (:Authority
      (bind _asplayer_controller_bp (Utilities|Casting|CastToPlayerController_BP NewPlayer))
      (Utilities|Array|Add (Variables|Default|GetPlayerControllerBPs) _asplayer_controller_bp)
      (bind _outactors (Actor|GetAllActorsOfClass "/Script/Engine.PlayerStart"))
      (Variables|Default|SetSpawnPoints _outactors)
      (CallFunction|RespawnPlayer _asplayer_controller_bp))))

(fn ConstructionScript)

(fn ToggleHUD
  (if (Variables|Default|GetMS_Showing)
    (Widget|RemovefromParent (Variables|Default|GetMS_widget))
    (Variables|Default|SetMS_Showing false)
    (else
      (UserInterface|Viewport|AddtoViewport (Variables|Default|GetMS_widget) 0)
      (Variables|Default|SetMS_Showing true))))