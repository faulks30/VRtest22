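; Player pawn Blueprint that handles planar movement and stepped left/right turning from input.
; MotionForward and MotionRight axes feed movement input along forward and right vectors built from control yaw only, ignoring pitch and roll.
; TurnLeft and TurnRight presses rotate the actor a quarter turn and also add fixed controller yaw input, which changes the heading used for movement.
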(event EventBeginPlay)

(event Collision|EventActorBeginOverlap
  (params (OtherActor :type Actor%20Object%20Reference)))

(event EventTick
  (params (DeltaSeconds :type Float%20%28single-precision%29)))

(event Input|ActionEvents|InputActionTurnLeft
  (params (Key :type Key%20Structure))
  (:Pressed
    (Transformation|AddActorLocalRotation "0,-90.000000, 0" false false)
    (Pawn|Input|AddControllerYawInput -36.0)))

(event Input|ActionEvents|InputActionTurnRight
  (params (Key :type Key%20Structure))
  (:Pressed
    (Transformation|AddActorLocalRotation "0,90.000000, 0" false false)
    (Pawn|Input|AddControllerYawInput 36.0)))

(event Input|AxisEvents|InputAxisMotionForward
  (params (AxisValue :type Float%20%28single-precision%29))
  (Pawn|Input|AddMovementInput (Math|Vector|GetForwardVector (Math|Rotator|MakeRotator 0.0 0.0 (.Yaw (Math|Rotator|BreakRotator (Pawn|GetControlRotation :!class /Script/Engine.Pawn))))) AxisValue false))

(event Input|AxisEvents|InputAxisMotionRight
  (params (AxisValue :type Float%20%28single-precision%29))
  (Pawn|Input|AddMovementInput (Math|Vector|GetRightVector (Math|Rotator|MakeRotator 0.0 0.0 (.Yaw (Math|Rotator|BreakRotator (Pawn|GetControlRotation :!class /Script/Engine.Pawn))))) AxisValue false))

(fn ConstructionScript)