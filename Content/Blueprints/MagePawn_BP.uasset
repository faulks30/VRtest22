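; Player pawn for the Mage, extending a parent pawn with mouse-driven sword combat and look controls.
; On authority, Tick interpolates the sword and passes its location and rotation to SwordCollisionParent through ServerSetLocationRotation.
; Attack input starts and stops combat.
; Off iOS, mouse axes steer the sword while blocking or attacking, otherwise turn the view and send yaw through ServerRotate.
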(event EventBeginPlay
  ;[1 1 1] Begin Play - set PawnType 2 (Mage)
  (|CallParentFunction))

(event EventTick
  (params (DeltaSeconds :type Float%20%28single-precision%29))
  ;[1 1 1] Tick - move hand around
  (|CallParentFunction DeltaSeconds)
  (Networking|SwitchHasAuthority
    (:Authority
      (bind (_new_location _new_rotation) (CallFunction|InterpolateSword DeltaSeconds))
      (CallFunction|ServerSetLocationRotation (Variables|Default|GetSword%20Collision%20Parent) _new_location _new_rotation false false))))

(event Input|ActionEvents|InputActionAttack
  (params (Key :type Key%20Structure))
  ;[1 1 1] Client - Draw/sheath sword
  (:Pressed
    (CallFunction|StartCombat))
  (:Released
    (CallFunction|StopCombat)))

(event Input|ActionEvents|InputActionBlock
  (params (Key :type Key%20Structure))
  ;[1 1 1] Client - Draw/sheath sword
)

(event Input|AxisEvents|InputAxisLookUp
  (params (AxisValue :type Float%20%28single-precision%29))
  (bind _playercontroller (Variables|Default|GetPlayerController))
  (bind (_locationx _locationy) (Game|Player|GetMousePosition _playercontroller))
  ;[1 1 1] Mouse Look
  (if (not (Variables|Default|GetIOS%20Game))
    (Variables|Default|SetMouse%20XY (Math|Vector2D|MakeVector2D _locationx _locationy))
    (bind _output_get (Variables|Default|SetOLD%20Mouse%20Delta%20Y AxisValue))
    (if (Variables|Default|GetBlocking)
      (CallFunction|MouseMoveSwordBlock)
      (elif (Variables|Default|GetCombat%20Mode)
        (CallFunction|MouseMoveSwordAttack)
        (else
          (Pawn|Input|AddControllerPitchInput _output_get))))))

(event Input|AxisEvents|InputAxisLookRight
  (params (AxisValue :type Float%20%28single-precision%29))
  (bind _playercontroller (Variables|Default|GetPlayerController))
  (bind (_locationx _locationy) (Game|Player|GetMousePosition _playercontroller))
  ;[1 1 1] Mouse Look
  (if (not (Variables|Default|GetIOS%20Game))
    (if (Variables|Default|GetUpdateMouseX)
      (Variables|Default|SetUpdateMouseX false)
      (else
        (Variables|Default|SetMouse%20XY (Math|Vector2D|MakeVector2D _locationx _locationy))
        (bind _output_get (Variables|Default|SetOLD%20Mouse%20Delta%20X AxisValue))
        (if (Variables|Default|GetBlocking)
          (CallFunction|MouseMoveSwordBlock)
          (elif (Variables|Default|GetCombat%20Mode)
            (CallFunction|MouseMoveSwordAttack)
            (else
              (Utilities|MyAddActorRotation (Math|Rotator|MakeRotator 0.0 0.0 (* _output_get 2.5))
                (:%20%20
                  (Pawn|Input|AddControllerYawInput _output_get)
                  (CallFunction|ResetMousetoMiddleScreen))))))))))

(fn ConstructionScript
  (|CallParentFunction))