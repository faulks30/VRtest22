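; Game mode that sets up platform flags, HUD widgets and the enemy list when play begins.
; BeginPlay flags iOS and VR on the player pawn, adds an iOS-only HUD, and shows the main HUD only without a connected headset.
; It also gathers ClawZombie and QueenVampire actors into EnemyActors and optionally opens the main menu through the game instance.
; Despite its name, ToggleHUD shows or hides the mission status widget.
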(event EventBeginPlay
  (bind _returnvalue (Game|GetPlayerController 0))
  (bind _returnvalue_2 (Game|GetPlatformName))
  (bind _returnvalue_3 (Class|HeadMountedDisplayFunctionLibrary|IsHeadMountedDisplayConnected))
  (bind _returnvalue_4 (Utilities|Enum|Equal(Enum) _returnvalue_2 "IOS"))
  ;[1 1 1] Create HUD, set platform variables
  (bind _asdefault_pawn_bp (Utilities|Casting|CastToDefaultPawn_BP (Game|GetPlayerCharacter 0)))
  (Variables|/Game/Blueprints/DefaultPawn_BP.DefaultPawn_BP_C|SetIOS%20Game _asdefault_pawn_bp _returnvalue_4)
  (Variables|/Game/Blueprints/DefaultPawn_BP.DefaultPawn_BP_C|SetVR%20Game _asdefault_pawn_bp _returnvalue_3)
  (if _returnvalue_4
    (bind _returnvalue_5 (UserInterface|CreateWidget "/Game/Blueprints/UI/IOS_HUD.IOS_HUD_C" _returnvalue))
    (bind _output_get (Variables|Default|SetHUD_IOS_Widget _returnvalue_5))
    (UserInterface|Viewport|AddtoViewport _output_get 0))
  (bind _returnvalue_6 (UserInterface|CreateWidget "/Game/Blueprints/UI/HUD.HUD_C" _returnvalue))
  (bind _output_get_2 (Variables|Default|SetHUD_Widget _returnvalue_6))
  (if _returnvalue_3
    _
    (else
      (UserInterface|Viewport|AddtoViewport _output_get_2 0)))
  (bind _returnvalue_7 (UserInterface|CreateWidget "/Game/Blueprints/UI/MissionStatus.MissionStatus_C" _returnvalue))
  (Variables|Default|SetMS_widget _returnvalue_7)
  (Variables|Default|SetMS_Showing false)
  (bind _outactors (Actor|GetAllActorsOfClass "/Game/Monsters/ClawZombie/ClawZombie.ClawZombie_C"))
  (Utilities|Array|AppendArray (Variables|Default|GetEnemy%20Actors) _outactors)
  (bind _outactors_2 (Actor|GetAllActorsOfClass "/Game/Monsters/QueenVampire/QueenVampire.QueenVampire_C"))
  (Utilities|Array|AppendArray (Variables|Default|GetEnemy%20Actors) _outactors_2)
  (if (Variables|Default|GetShowMenu)
    (bind _asgame_instance_bp (Utilities|Casting|CastToGameInstanceBP (Game|GetGameInstance)))
    (Default|ShowMainMenu _asgame_instance_bp)))

(fn ConstructionScript)

(fn ToggleHUD
  (if (Variables|Default|GetMS_Showing)
    (Widget|RemovefromParent (Variables|Default|GetMS_widget))
    (Variables|Default|SetMS_Showing false)
    (else
      (UserInterface|Viewport|AddtoViewport (Variables|Default|GetMS_widget) 0)
      (Variables|Default|SetMS_Showing true))))