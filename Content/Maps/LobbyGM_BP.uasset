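; LobbyGM_BP is the lobby Blueprint, likely a game mode, that marks lobby state and toggles an on-screen widget.
; Its construction script casts the game instance to GameInstanceBP and sets InLobby to true.
; ToggleHUD adds MSWidget to the viewport or removes it from its parent, tracking visibility in the MSShowing flag.
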(fn ConstructionScript
  (bind _asgame_instance_bp (Utilities|Casting|CastToGameInstanceBP (Game|GetGameInstance)))
  (Variables|/Game/Blueprints/GameInstanceBP.GameInstanceBP_C|SetInLobby _asgame_instance_bp true))

(fn ToggleHUD
  (if (Variables|Default|GetMS_Showing)
    (Widget|RemovefromParent (Variables|Default|GetMS_widget))
    (Variables|Default|SetMS_Showing false)
    (else
      (UserInterface|Viewport|AddtoViewport (Variables|Default|GetMS_widget) 0)
      (Variables|Default|SetMS_Showing true))))