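; Map game mode that tracks enemies and handles player spawning.
; At BeginPlay it gathers all ClawZombie and QueenVampire actors into an enemy list.
; On authority, PostLogin records each new player controller, collects the map's PlayerStarts and calls RespawnPlayer.
; RespawnPlayer spawns a DefaultPawn_BP at a random start, adjusting for collisions, and has the controller possess it.
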(event Custom|RespawnPlayer
  (params (PlayerController :type Player%20Controller%20BP%20Object%20Reference))
  (bind _spawnpoints (Variables|Default|GetSpawnPoints))
  ;[1 1 1] Respawn new player
  (Utilities|IsValid (Pawn|GetControlledPawn PlayerController)
    (:Is%20Valid
      (Actor|DestroyActor))
    (:Is%20Not%20Valid
      _))
  (bind _returnvalue (Game|SpawnActorfromClass "/Game/Blueprints/DefaultPawn_BP.DefaultPawn_BP_C" (Transformation|GetActorTransform (Utilities|Array|Get(acopy) _spawnpoints (Math|Random|RandomIntegerinRange 0 (- (Utilities|Array|Length _spawnpoints) 1)))) "AdjustIfPossibleButAlwaysSpawn" 0 0))
  (Pawn|Possess PlayerController _returnvalue))

(event EventBeginPlay
  ;[1 1 1] Create HUD, set platform variables
  (bind _outactors (Actor|GetAllActorsOfClass "/Game/Monsters/ClawZombie/ClawZombie.ClawZombie_C"))
  (Utilities|Array|AppendArray (Variables|Default|GetEnemy%20Actors) _outactors)
  (bind _outactors_2 (Actor|GetAllActorsOfClass "/Game/Monsters/QueenVampire/QueenVampire.QueenVampire_C"))
  (Utilities|Array|AppendArray (Variables|Default|GetEnemy%20Actors) _outactors_2))

(event EventPostLogin
  (params (NewPlayer :type Player%20Controller%20Object%20Reference))
  ;[1 1 1] New player logged on
  (Networking|SwitchHasAuthority
    (:Authority
      (bind _asplayer_controller_bp (Utilities|Casting|CastToPlayerController_BP NewPlayer))
      (Utilities|Array|Add (Variables|Default|GetPlayerControllerBPs) _asplayer_controller_bp)
      (bind _outactors (Actor|GetAllActorsOfClass "/Script/Engine.PlayerStart"))
      (Variables|Default|SetSpawnPoints _outactors)
      (CallFunction|RespawnPlayer _asplayer_controller_bp))))

(fn ConstructionScript)